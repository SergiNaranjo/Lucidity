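; Interactable door that swings open and closes itself, usable only once the game instance's Submitted flag is set.
; Player overlap checks that flag on Lucidity_GM, cast from the game instance, to enable interaction; leaving disables it.
; IA_Interact rotates the Scene component 90 degrees through chained short Delays instead of a Timeline, pauses briefly, then steps it back closed.
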(event `self.ReceiveBeginPlay`
  (`self.SetActorHiddenInGame` false)
  (`self.SetActorEnableCollision` true)
  (`self.EnableInput` (`GameplayStatics.GetPlayerController` 0)))

(event `self.ReceiveActorBeginOverlap`
  (params (OtherActor :type "Actor Object Reference"))
  (if (== OtherActor (`GameplayStatics.GetPlayerCharacter` 0))
    (bind _aslucidity_gm (cast `/Game/Lucidity_GM` (`GameplayStatics.GetGameInstance`)))
    (if (`/Game/Lucidity_GM.Submitted` _aslucidity_gm)
      (set `self.CanInteract` true))))

(event `self.ReceiveActorEndOverlap`
  (params (OtherActor :type "Actor Object Reference"))
  (if (== OtherActor (`GameplayStatics.GetPlayerCharacter` 0))
    (set `self.CanInteract` false)))

(event `EnhancedInput|/Game/FirstPerson/Input/Actions/IA_Interact`
  (params (ActionValue :type Boolean) (ElapsedSeconds :type "Float (double-precision)") (TriggeredSeconds :type "Float (double-precision)") (InputAction :type "InputAction Object Reference" :default "/Game/FirstPerson/Input/Actions/IA_Interact.IA_Interact"))
  (:`Triggered`
    (if (== (`self.CanInteract`) true)
      (`SceneComponent.K2_SetRelativeRotation` (`self.Scene`) (struct :`Yaw` -10.0) false false)
      (`KismetSystemLibrary.Delay` 0.01)
      (`SceneComponent.K2_SetRelativeRotation` (`self.Scene`) (struct :`Yaw` -20.0) false false)
      (`KismetSystemLibrary.Delay` 0.01)
      (`SceneComponent.K2_SetRelativeRotation` (`self.Scene`) (struct :`Yaw` -30.0) false false)
      (`KismetSystemLibrary.Delay` 0.01)
      (`SceneComponent.K2_SetRelativeRotation` (`self.Scene`) (struct :`Yaw` -40.0) false false)
      (`KismetSystemLibrary.Delay` 0.01)
      (`SceneComponent.K2_SetRelativeRotation` (`self.Scene`) (struct :`Yaw` -50.0) false false)
      (`KismetSystemLibrary.Delay` 0.01)
      (`SceneComponent.K2_SetRelativeRotation` (`self.Scene`) (struct :`Yaw` -60.0) false false)
      (`KismetSystemLibrary.Delay` 0.01)
      (`SceneComponent.K2_SetRelativeRotation` (`self.Scene`) (struct :`Yaw` -70.0) false false)
      (`KismetSystemLibrary.Delay` 0.01)
      (`SceneComponent.K2_SetRelativeRotation` (`self.Scene`) (struct :`Yaw` -80.0) false false)
      (`KismetSystemLibrary.Delay` 0.01)
      (`SceneComponent.K2_SetRelativeRotation` (`self.Scene`) (struct :`Yaw` -90.0) false false)
      (`KismetSystemLibrary.Delay` 1.2)
      (`SceneComponent.K2_SetRelativeRotation` (`self.Scene`) (struct :`Yaw` -80.0) false false)
      (`KismetSystemLibrary.Delay` 0.01)
      (`SceneComponent.K2_SetRelativeRotation` (`self.Scene`) (struct :`Yaw` -70.0) false false)
      (`KismetSystemLibrary.Delay` 0.01)
      (`SceneComponent.K2_SetRelativeRotation` (`self.Scene`) (struct :`Yaw` -60.0) false false)
      (`KismetSystemLibrary.Delay` 0.01)
      (`SceneComponent.K2_SetRelativeRotation` (`self.Scene`) (struct :`Yaw` -50.0) false false)
      (`KismetSystemLibrary.Delay` 0.01)
      (`SceneComponent.K2_SetRelativeRotation` (`self.Scene`) (struct :`Yaw` -40.0) false false)
      (`KismetSystemLibrary.Delay` 0.01)
      (`SceneComponent.K2_SetRelativeRotation` (`self.Scene`) (struct :`Yaw` -30.0) false false)
      (`KismetSystemLibrary.Delay` 0.01)
      (`SceneComponent.K2_SetRelativeRotation` (`self.Scene`) (struct :`Yaw` -20.0) false false)
      (`KismetSystemLibrary.Delay` 0.01)
      (`SceneComponent.K2_SetRelativeRotation` (`self.Scene`) (struct :`Yaw` -10.0) false false)
      (`KismetSystemLibrary.Delay` 0.01)
      (`SceneComponent.K2_SetRelativeRotation` :`self` (`self.Scene`)))))

(fn `UserConstructionScript`)