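; DoorLoop_BP is an interactable door actor that sends the player back to a referenced StartPoint.
; Player overlap toggles a CanTeleport flag that gates the IA_Interact input, enabled on the actor at BeginPlay.
; Interacting moves the character to StartPoint's location without sweep and matches the control rotation to its rotation.
; The actor's visibility and collision are switched off just before the move and restored immediately afterwards.
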(event `self.ReceiveBeginPlay`
  (`self.SetActorHiddenInGame` false)
  (`self.SetActorEnableCollision` true)
  (`self.EnableInput` (`GameplayStatics.GetPlayerController` 0)))

(event `self.ReceiveActorBeginOverlap`
  (params (OtherActor :type "Actor Object Reference"))
  (if (== OtherActor (`GameplayStatics.GetPlayerCharacter` 0))
    (set `self.CanTeleport` true)))

(event `self.ReceiveActorEndOverlap`
  (params (OtherActor :type "Actor Object Reference"))
  (if (== OtherActor (`GameplayStatics.GetPlayerCharacter` 0))
    (set `self.CanTeleport` false)))

(event `EnhancedInput|/Game/FirstPerson/Input/Actions/IA_Interact`
  (params (ActionValue :type Boolean) (ElapsedSeconds :type "Float (double-precision)") (TriggeredSeconds :type "Float (double-precision)") (InputAction :type "InputAction Object Reference" :default "/Game/FirstPerson/Input/Actions/IA_Interact.IA_Interact"))
  (bind _startpoint (`self.StartPoint`))
  (:`Triggered`
    (if (== (`self.CanTeleport`) true)
      (`self.SetActorHiddenInGame` true)
      (`self.SetActorEnableCollision` false)
      (`self.K2_SetActorLocation` (`GameplayStatics.GetPlayerCharacter` 0) (`self.K2_GetActorLocation` (`|ConvertAsset` _startpoint)) false false)
      (`Controller.SetControlRotation` (`GameplayStatics.GetPlayerController` 0) (`self.K2_GetActorRotation` (`|ConvertAsset` _startpoint)))
      (`self.SetActorHiddenInGame` false)
      (`self.SetActorEnableCollision` true))))

(fn `UserConstructionScript`)